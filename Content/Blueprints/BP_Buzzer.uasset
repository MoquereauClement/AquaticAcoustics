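; BP_Buzzer is a buzzer button that can be hovered, pressed and released.
; Hovering swaps the button mesh between idle and hover materials.
; Pressing snaps the mesh down by PressDepth from the location cached at BeginPlay, guarded against repeat presses, and release restores it.
; Press and release only print debug messages besides the visual change and state flag, and nothing in this Blueprint calls these events.
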(event Custom|SetHovered
  (params (Hovered :type Boolean))
  (bind _output_get (Variables|Default|SetbIsHovered Hovered))
  (if _output_get
    (Rendering|Material|SetMaterial (Variables|Default|GetButtonMesh) 0 (Variables|Default|GetHoverMaterial))
    (else
      (Rendering|Material|SetMaterial (Variables|Default|GetButtonMesh) 0 (Variables|Default|GetIdleMaterial)))))

(event Custom|ReleaseBuzzer
  (Variables|Default|SetbIsPressed false)
  (Transformation|SetRelativeLocation (Variables|Default|GetButtonMesh) (Variables|Default|GetButtonInitialLocation) false false)
  (Development|PrintString "Buzzer Relaché!"))

(event Custom|PressBuzzer
  (bind _buttoninitiallocation (Variables|Default|GetButtonInitialLocation))
  (bind (_x _y _z) (Math|Vector|BreakVector _buttoninitiallocation))
  (if (not (Variables|Default|GetbIsPressed))
    (Variables|Default|SetbIsPressed true)
    (Transformation|SetRelativeLocation (Variables|Default|GetButtonMesh) (Math|Vector|MakeVector _x _y (- _z (Variables|Default|GetPressDepth))) false false)
    (Development|PrintString "Buzzer Actif!")))

(event EventBeginPlay
  (Variables|Default|SetButtonInitialLocation (Variables|/Script/Engine.SceneComponent|GetRelativeLocation (Variables|Default|GetButtonMesh))))

(fn ConstructionScript)